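; BP_Bacteria is a bacteria actor that reacts to overlapping water molecules by consuming them and releasing bacteria molecules.
; On overlap with a BP_WaterMol, it destroys the molecule and calls ReduceWater on the BP_CharacterControler found in the level.
; It then spawns three BP_BacteriaMol actors stacked upward with random horizontal offsets and destroys itself.
; A separate DigRock function only prints a debug message and destroys the actor.
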(event `self.ReceiveActorBeginOverlap`
  (params (OtherActor :type "Actor Object Reference"))
  (bind _returnvalue (`self.GetTransform`))
  (bind _returnvalue_2 (* (`KismetMathLibrary.RandomFloat`) 20.0))
  (bind _asbp_water_mol (cast `/Game/BluePrints/BP_WaterMol` OtherActor))
  (`self.K2_DestroyActor` _asbp_water_mol)
  (bind _returnvalue_3 (`GameplayStatics.GetActorOfClass` "/Game/BluePrints/BP_CharacterControler.BP_CharacterControler_C"))
  (`/Game/BluePrints/BP_CharacterControler.ReduceWater` _returnvalue_3)
  (for _index (range 3)
    (`|SpawnActorFromClass` "/Game/BluePrints/BP_BacteriaMol.BP_BacteriaMol_C" (`KismetMathLibrary.MakeTransform` (`KismetMathLibrary.MakeVector` (+ (.x (.location _returnvalue)) _returnvalue_2) (+ _returnvalue_2 (.y (.location _returnvalue))) (+ (* _index 20) (.z (.location _returnvalue)))) (.rotation _returnvalue) (.scale _returnvalue)) "Undefined" "MultiplyWithRoot" null null))
  (`self.K2_DestroyActor`))

(fn `DigRock`
  (`KismetSystemLibrary.PrintString` "Rock Dug")
  (`self.K2_DestroyActor`))

(fn `UserConstructionScript`)