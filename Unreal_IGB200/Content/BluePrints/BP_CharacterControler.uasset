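; Player controller for a touch-driven digging game that routes taps to blocks and tracks win and lose counts.
; BeginPlay adds the mobile input mapping, sets the first managed camera, and derives pyrite and water counts from placed acid and water blocks.
; Taps trace after a retriggerable delay, ignoring invisible walls, to rock, acid or water blocks.
; ReducePyrite and ReduceWater show win or lose at zero; ChangeCameraView cycles cameras, but the double-tap branch is empty.
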(event `self.ReceiveBeginPlay`
  ;[1 1 1] Add Controls
  (bind _asplayer_controller (cast `PlayerController` (`GameplayStatics.GetPlayerController` 0)))
  (bind _returnvalue (pcsubsystem `EnhancedInputLocalPlayerSubsystem` _asplayer_controller))
  (`/Engine/EditorBlueprintResources/StandardMacros.IsValid` _returnvalue
    (:`Is Valid`
      (`EnhancedInputSubsystemInterface.AddMappingContext` _returnvalue "/Game/Input/IMC_Mobile.IMC_Mobile" 0 (struct))
      ;[1 1 1] Set Main Camera
      (bind _outactors (`GameplayStatics.GetAllActorsOfClass` "/Script/Engine.CameraActor"))
      (bind _output_get (set `self.MainCamera` (`|GetArrayItem` _outactors)))
      (`self.SetViewTargetWithBlend` _output_get)
      ;[1 1 1] Set Camera
      (bind _outactors_2 (`GameplayStatics.GetAllActorsOfClass` "/Game/BluePrints/BP_CameraManager.BP_CameraManager_C"))
      (bind _output_get_2 (set `self.Cameras` (`/Game/BluePrints/BP_CameraManager.Cameras` (`|GetArrayItem` _outactors_2))))
      (`self.SetViewTargetWithBlend` (`|GetArrayItem` _output_get_2))
      ;[1 1 1] Set Water Count
      (bind _outactors_3 (`GameplayStatics.GetAllActorsOfClass` "/Game/BluePrints/BP_WaterBlock.BP_WaterBlock_C"))
      (set `self.WaterCount` (* (`KismetArrayLibrary.Array_Length` _outactors_3) 5))
      ;[1 1 1] Set Pyrite Count
      (bind _outactors_4 (`GameplayStatics.GetAllActorsOfClass` "/Game/BluePrints/BP_AcidBlock.BP_AcidBlock_C"))
      (set `self.PyriteCount` (`KismetArrayLibrary.Array_Length` _outactors_4))
      ;[1 1 1] Get Invisible Walls
      (bind _outactors_5 (`GameplayStatics.GetAllActorsOfClass` "/Game/BluePrints/BP_InvisibleWall.BP_InvisibleWall_C"))
      (set `self.InvisbleWalls` _outactors_5))))

(event `Key|Touch1` :consume false
  (params (Key :type "Key Structure"))
  (bind (_returnvalue_x _returnvalue_y) (`KismetMathLibrary.BreakVector` (`self.GetInputVectorKeyState` Key)))
  (bind _clickcounter (`self.ClickCounter`))
  (bind (_worldposition _worlddirection) (`GameplayStatics.DeprojectScreenToWorld` self (`KismetMathLibrary.MakeVector2D` _returnvalue_x _returnvalue_y)))
  (:`Pressed`
    (`|ExecutionSequence`
      (:`then_0`
        (`/Engine/EditorBlueprintResources/StandardMacros.IncrementInt` _clickcounter
          (:`  `
            (if (>= _clickcounter 2)
              _))))
      (:`then_1`
        (`KismetSystemLibrary.RetriggerableDelay` 0.2)
        (set `self.ClickCounter` 0)
        ;[1 1 1] Raycast For Objects
        (bind _outhit (`KismetSystemLibrary.LineTraceSingleForObjects` _worldposition (+ _worldposition (* _worlddirection 100000.0)) (`|MakeArray` "ObjectTypeQuery2" :!type "EObjectTypeQuery Enum") false (`self.InvisbleWalls`)))
        (bind _asbp_rock_diggable (cast `/Game/BluePrints/BP_RockDiggable` (`.HitActor` (`GameplayStatics.BreakHitResult` _outhit)))
          (:`then`
            (`/Game/BluePrints/BP_RockDiggable.DigRock` _asbp_rock_diggable))
          (:`CastFailed`
            (bind _asbp_acid_block (cast `/Game/BluePrints/BP_AcidBlock` (`.HitActor` (`GameplayStatics.BreakHitResult` _outhit)))
              (:`then`
                (`/Game/BluePrints/BP_AcidBlock.DigAcid` _asbp_acid_block))
              (:`CastFailed`
                (bind _asbp_water_block (cast `/Game/BluePrints/BP_WaterBlock` (`.HitActor` (`GameplayStatics.BreakHitResult` _outhit))))
                (`/Game/BluePrints/BP_WaterBlock.TouchWater` _asbp_water_block)))))))))

(event `Key|Escape`
  (params (Key :type "Key Structure"))
  (:`Pressed`
    (`KismetSystemLibrary.QuitGame` null "Quit")))

(fn `Change Camera View`
  (`KismetSystemLibrary.PrintString` "Double Touch")
  (if (>= (`self.CameraIndex`) (- (`KismetArrayLibrary.Array_Length` (`self.Cameras`)) 1))
    (set `self.CameraIndex` 0)
    (else
      (`/Engine/EditorBlueprintResources/StandardMacros.IncrementInt` (`self.CameraIndex`)
        (:`  `
          _))))
  (`self.SetViewTargetWithBlend` (`|GetArrayItem` (`self.Cameras`) (`self.CameraIndex`)) 0.1))

(fn `ReducePyrite`
  (bind _result (`/Engine/EditorBlueprintResources/StandardMacros.DecrementInt` (`self.PyriteCount`))
    (:`  `
      (`KismetSystemLibrary.PrintString` (`KismetStringLibrary.Conv_IntToString` _result))
      (if (== (`self.PyriteCount`) 0)
        (bind _returnvalue (`|CreateWidget` "/Game/BluePrints/UI_BluePrints/BP_Win.BP_Win_C"))
        (`UserWidget.AddToViewport` _returnvalue 0)))))

(fn `ReduceWater`
  (bind _result (`/Engine/EditorBlueprintResources/StandardMacros.DecrementInt` (`self.WaterCount`))
    (:`  `
      (`KismetSystemLibrary.PrintString` (`KismetStringLibrary.Conv_IntToString` _result))
      (if (== (`self.WaterCount`) 0)
        (bind _returnvalue (`|CreateWidget` "/Game/BluePrints/UI_BluePrints/BP_Lose.BP_Lose_C"))
        (`UserWidget.AddToViewport` _returnvalue 0)))))

(fn `UserConstructionScript`)