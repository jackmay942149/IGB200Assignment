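; BP_AcidMol is a physics-driven acid molecule that steers itself around static obstacles as if carried by flowing water.
; CalculateDirectionOfForce line-traces along world +X, +Y and -Y, packing open paths into a vector's components as flags.
; Tick pushes the Sphere by WaterSpeed and delta time, preferring forward, then sideways according to TravellingRight.
; RandomChangeBool occasionally flips that side preference during sideways movement, with debug prints throughout.
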(event `self.ReceiveTick`
  (params (DeltaSeconds :type "Float (single-precision)"))
  (set `self.ForceMulti` (* (* DeltaSeconds (`self.WaterSpeed`)) 1000.0))
  (bind _force (`self.CalculateDirectionOfForce`))
  (if (> (.x _force) 0.0)
    (`PrimitiveComponent.AddForce` (`self.Sphere`) (`KismetMathLibrary.MakeVector` (`self.ForceMulti`)) "None" false)
    (`KismetSystemLibrary.PrintString` "Moving Forward")
    (elif (and (> (.y _force) 0.0) (`self.TravellingRight`))
      (`PrimitiveComponent.AddForce` (`self.Sphere`) (`KismetMathLibrary.MakeVector` 0.0 (`self.ForceMulti`)) "None" false)
      (`KismetSystemLibrary.PrintString` "Moving Right")
      (`self.RandomChangeBool` (`self.TravellingRight`) 1000 :!label _label)
      (elif (> (.z _force) 0.0)
        (set `self.TravellingRight` false)
        (`PrimitiveComponent.AddForce` (`self.Sphere`) (`KismetMathLibrary.MakeVector` 0.0 (* (`self.ForceMulti`) -1.0)) "None" false)
        (`KismetSystemLibrary.PrintString` "Moving Left")
        (goto _label)
        (else
          (set `self.TravellingRight` true)
          (`KismetSystemLibrary.PrintString` "Not Moving"))))))

(fn `CalculateDirectionOfForce`
  (returns (Force :type "Vector Structure"))
  (locals (ForceToReturn :type "Vector Structure"))
  (bind (_forcetoreturn_x _forcetoreturn_y _forcetoreturn_z) (`KismetMathLibrary.BreakVector` (`local.ForceToReturn`)))
  (bind (_forcetoreturn_x_2 _forcetoreturn_y_2 _forcetoreturn_z_2) (`KismetMathLibrary.BreakVector` (`local.ForceToReturn`)))
  (bind _returnvalue (`SceneComponent.K2_GetComponentLocation` (`self.Sphere`)))
  (bind _returnvalue_2 (`SceneComponent.K2_GetComponentLocation` (`self.Sphere`)))
  (bind _returnvalue_3 (`SceneComponent.K2_GetComponentLocation` (`self.Sphere`)))
  ;[1 1 1] Raycast Forward
  (bind (_outhit _returnvalue_4) (`KismetSystemLibrary.LineTraceSingleForObjects` :`Start` _returnvalue_3 :`End` (`KismetMathLibrary.MakeVector` (+ (`self.NavRayDist`) (.x _returnvalue_3)) (.y _returnvalue_3) (.z _returnvalue_3)) :`ObjectTypes` (`|MakeArray` "ObjectTypeQuery1" :!type "EObjectTypeQuery Enum") :`DrawTime` 1.0))
  ;[1 1 1] Raycast Right
  (bind (_outhit_2 _returnvalue_5) (`KismetSystemLibrary.LineTraceSingleForObjects` :`Start` _returnvalue_2 :`End` (`KismetMathLibrary.MakeVector` (.x _returnvalue_2) (+ (.y _returnvalue_2) (`self.NavRayDist`)) (.z _returnvalue_2)) :`ObjectTypes` (`|MakeArray` "ObjectTypeQuery1" :!type "EObjectTypeQuery Enum") :`DrawTime` 1.0))
  ;[1 1 1] Raycast Left
  (bind (_outhit_3 _returnvalue_6) (`KismetSystemLibrary.LineTraceSingleForObjects` :`Start` _returnvalue :`End` (`KismetMathLibrary.MakeVector` (.x _returnvalue) (- (.y _returnvalue) (`self.NavRayDist`)) (.z _returnvalue)) :`ObjectTypes` (`|MakeArray` "ObjectTypeQuery1" :!type "EObjectTypeQuery Enum") :`DrawTime` 1.0))
  (if _returnvalue_4
    (set `local.ForceToReturn` (0.0 0.0 0.0))
    (else
      (set `local.ForceToReturn` (1.0 0.0 0.0))))
  (if (not _returnvalue_5)
    (set `local.ForceToReturn` (`KismetMathLibrary.MakeVector` _forcetoreturn_x_2 (+ _forcetoreturn_y_2 1.0) _forcetoreturn_z_2)))
  (if (not _returnvalue_6)
    (set `local.ForceToReturn` (`KismetMathLibrary.MakeVector` _forcetoreturn_x _forcetoreturn_y (+ _forcetoreturn_z 1.0))))
  (return (`local.ForceToReturn`)))

(fn `RandomChangeBool`
  (params (theBool :type "Boolean (by ref)") (Chance :type Integer))
  (if (not (> (`KismetMathLibrary.RandomInteger` Chance) 0))
    (`|VariableSetRef` theBool (not theBool))
    (`KismetSystemLibrary.PrintString` "Changed Direction" true true (struct :`R` 1.0 :`B` 0.057139 :`A` 1.0)))
  (return))

(fn `UserConstructionScript`)