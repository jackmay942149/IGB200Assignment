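; BP_StibBlock is a diggable block that penalizes the player when water or bacteria molecules overlap it.
; Either overlap plays a sound, lowers the BP_CharacterControler score and destroys both actors.
; Water also reduces the water count and triggers force feedback, while bacteria reduces pyrite and costs more score, despite its success sound.
; DigRock prints a debug string and destroys the block; DigAcid is an empty stub.
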(event `self.ReceiveActorBeginOverlap`
  (params (OtherActor :type "Actor Object Reference"))
  (bind _asbp_water_mol (cast `/Game/BluePrints/BP_WaterMol` OtherActor)
    (:`then`
      (`GameplayStatics.PlaySoundAtLocation` "/Game/Sounds/lose_sound.lose_sound" (`self.K2_GetActorLocation`) (struct) 1.0 1.0 0.0 null null null null)
      (bind _returnvalue (`GameplayStatics.GetActorOfClass` "/Game/BluePrints/BP_CharacterControler.BP_CharacterControler_C"))
      (`/Engine/EditorBlueprintResources/StandardMacros.DecrementInt` (`/Game/BluePrints/BP_CharacterControler.Score` _returnvalue)
        (:`  `
          (`/Game/BluePrints/BP_CharacterControler.ReduceWater` _returnvalue)
          (`self.K2_DestroyActor` _asbp_water_mol)
          (`PlayerController.PlayDynamicForceFeedback` (`GameplayStatics.GetPlayerController` 0) 1.0 1.0 true true true true)
          (`self.K2_DestroyActor`))))
    (:`CastFailed`
      (bind _asbp_bacteria_mol (cast `/Game/BluePrints/BP_BacteriaMol` OtherActor))
      (`GameplayStatics.PlaySoundAtLocation` "/Game/Sounds/short-success-sound-glockenspiel-treasure-video-game-6346.short-success-sound-glockenspiel-treasure-video-game-6346" (`self.K2_GetActorLocation`) (struct) 1.0 1.0 0.0 null null null null)
      (bind _returnvalue_2 (`GameplayStatics.GetActorOfClass` "/Game/BluePrints/BP_CharacterControler.BP_CharacterControler_C"))
      (`/Game/BluePrints/BP_CharacterControler.ReducePyrite` _returnvalue_2)
      (set `/Game/BluePrints/BP_CharacterControler.Score` (- (`/Game/BluePrints/BP_CharacterControler.Score` _returnvalue_2) 3) _returnvalue_2)
      (`self.K2_DestroyActor` _asbp_bacteria_mol)
      (`self.K2_DestroyActor`))))

(fn `DigAcid`)

(fn `DigRock`
  (`KismetSystemLibrary.PrintString` "Rock Dug")
  (`self.K2_DestroyActor`))

(fn `UserConstructionScript`)