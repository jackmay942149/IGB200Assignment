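; BP_LevelGenerator is a level generator actor that defines a rectangular block area and can spawn diggable rock.
; The construction script rebuilds a spline as a four-point, linear-cornered rectangle, sized from the X and Y block counts at 100 units each, less TestFactor.
; A separate Spawner function spawns a BP_RockDiggable at a given position, but nothing in this file calls it and the event graph is inactive.
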(fn `Spawner`
  (params (SpawnPos :type "Vector Structure"))
  (`|SpawnActorFromClass` "/Game/BluePrints/BP_RockDiggable.BP_RockDiggable_C" (`KismetMathLibrary.MakeTransform` SpawnPos) "Undefined" "MultiplyWithRoot" null null))

(fn `UserConstructionScript`
  (bind _returnvalue (`KismetMathLibrary.Vector_Zero`))
  (bind _testfactor (`self.TestFactor`))
  (bind _returnvalue_2 (+ _returnvalue (`KismetMathLibrary.MakeVector` (`KismetMathLibrary.Conv_IntToDouble` (`self.Length`)))))
  (if (not false)
    (set `self.Length` (- (* (`self.BlockCountX`) 100) _testfactor))
    (set `self.Width` (- (* (`self.BlockCountY`) 100) _testfactor))
    (`SplineComponent.ClearSplinePoints` (`self.Spline`) true)
    (`SplineComponent.SetSplinePoints` (`self.Spline`) (`|MakeArray` _returnvalue _returnvalue_2 (+ _returnvalue_2 (`KismetMathLibrary.MakeVector` 0.0 (`KismetMathLibrary.Conv_IntToDouble` (`self.Width`)))) (+ _returnvalue (`KismetMathLibrary.MakeVector` 0.0 (`KismetMathLibrary.Conv_IntToDouble` (`self.Width`))))) "Local" true)
    (for _index (range 4)
      (`SplineComponent.SetSplinePointType` (`self.Spline`) _index "Linear" true))))